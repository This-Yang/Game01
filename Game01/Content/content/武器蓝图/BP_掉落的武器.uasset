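; Dropped weapon actor that lies in the world as a physics-simulated static mesh, configured by a weapon data asset.
; On authority only, the construction script takes the mesh from the asset and sets the current bullet count to its capacity.
; Highlight events apply or clear an interaction overlay material, and a getter returns the data asset.
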(event EventBeginPlay
  (Physics|SetSimulatePhysics (Variables|Default|GetStaticMesh) true))

(event Collision|EventActorBeginOverlap
  (params (OtherActor :type Actor%20Object%20Reference)))

(event EventTick
  (params (DeltaSeconds :type Float%20%28single-precision%29)))

(event Event关闭高亮
  (Rendering|Material|SetOverlayMaterial (Variables|Default|GetStaticMesh) 0 :!class /Script/Engine.MeshComponent))

(event Event高亮显示
  (Rendering|Material|SetOverlayMaterial (Variables|Default|GetStaticMesh) "/Game/Content/材质/M_交互材质.M_交互材质" :!class /Script/Engine.MeshComponent))

(fn ConstructionScript
  (Networking|SwitchHasAuthority
    (:Authority
      (Components|StaticMesh|SetStaticMesh (Variables|Default|GetStaticMesh) (Variables|/Game/Content/数据资产/武器数据资产/武器_数据资产.武器_数据资产_C|Get静态 (Variables|Default|Get武器数据资产)))
      (Variables|Default|Set当前子弹数量 (Variables|/Game/Content/数据资产/武器数据资产/武器_数据资产.武器_数据资产_C|Get容量 (Variables|Default|Get武器数据资产))))))

(fn 获取数据资产
  (return (Variables|Default|Get武器数据资产)))