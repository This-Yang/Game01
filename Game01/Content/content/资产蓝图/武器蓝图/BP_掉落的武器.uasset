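; Dropped weapon pickup that simulates physics, toggles an interaction overlay material for highlighting, and exposes its weapon data asset.
; On authority, construction takes the mesh and initial ammo count from that data asset.
; The skill cooldown runs on authority by playing a timeline, sized from the asset, in reverse from the stored remaining time if the skill is not ready.
; The update event stores the playback position and marks the skill ready at zero.
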(event Event关闭高亮
  (Rendering|Material|SetOverlayMaterial (Variables|Default|GetStaticMesh) 0 :!class /Script/Engine.MeshComponent))

(event Event高亮显示
  (Rendering|Material|SetOverlayMaterial (Variables|Default|GetStaticMesh) "/Game/content/材质/M_交互材质.M_交互材质" :!class /Script/Engine.MeshComponent))

(event Custom|进入CD
  (bind _cd (Variables|Default|GetCD))
  (Components|Timeline|SetPlaybackPosition _cd (Variables|Default|Get技能剩余CD) false false)
  (Utilities|String|Reverse _cd))

(event Custom|更新剩余CD
  (bind _output_get (Variables|Default|Set技能剩余CD (Components|Timeline|GetPlaybackPosition (Variables|Default|GetCD))))
  (if (<= _output_get 0.0)
    (Variables|Default|Set技能是否就绪 true)))

(event EventBeginPlay
  (bind _cd (Variables|Default|GetCD))
  (Networking|SwitchHasAuthority
    (:Authority
      (Components|Timeline|SetTimelineLength _cd (Variables|/Game/content/数据资产/武器数据资产/WP_数据资产.WP_数据资产_C|GetCD (Variables|Default|Get武器数据资产)))
      (Class|TimelineComponent|SetTimelinePostUpdateFunc _cd (EventDispatchers|CreateEvent :!event Custom|更新剩余CD))
      (if (not (Variables|Default|Get技能是否就绪))
        (CallFunction|进入CD)))))

(fn ConstructionScript
  (Networking|SwitchHasAuthority
    (:Authority
      (Components|StaticMesh|SetStaticMesh (Variables|Default|GetStaticMesh) (Variables|/Game/content/数据资产/武器数据资产/WP_数据资产.WP_数据资产_C|Get静态 (Variables|Default|Get武器数据资产)))
      (Variables|Default|Set当前子弹数量 (Variables|/Game/content/数据资产/武器数据资产/WP_数据资产.WP_数据资产_C|Get容量 (Variables|Default|Get武器数据资产))))
    (:Remote
      _))
  (Physics|SetSimulatePhysics (Variables|Default|GetStaticMesh) true))

(fn 获取数据资产
  (return (Variables|Default|Get武器数据资产)))