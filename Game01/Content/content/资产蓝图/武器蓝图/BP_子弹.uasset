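; BP_子弹 (bullet) resolves a shot's impact with surface-specific effects and point damage.
; Its Hit event runs a small sphere trace at the supplied location, choosing an impact particle by physical surface.
; Default, metal, concrete and wood surfaces also get a temporary bullet-hole decal.
; On a successful trace, only authority applies damage, credited to the damage source, and the actor destroys itself after a short delay.
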(event Collision|EventHit
  (params (MyComp :type Primitive%20Component%20Object%20Reference) (Other :type Actor%20Object%20Reference) (OtherComp :type Primitive%20Component%20Object%20Reference) (bSelfMoved :type Boolean) (HitLocation :type Vector :default "0, 0, 0") (HitNormal :type Vector :default "0, 0, 0") (NormalImpulse :type Vector :default "0, 0, 0") (Hit :type Hit%20Result%20Structure%20%28by%20ref%29))
  (bind _伤害来源 (Variables|Default|Get伤害来源))
  (bind (_outhit _returnvalue) (Collision|SphereTraceByChannel HitLocation HitLocation 3.0 "TraceTypeQuery6" false 0 "None"))
  (bind _output_get (Variables|Default|Set命中结果 _outhit))
  (if _returnvalue
    (switch Utilities|FlowControl|Switch|SwitchonEPhysicalSurface (Collision|GetSurfaceType _output_get)
      (:SurfaceType_Default
        (Variables|Default|Set击中特效 "/Game/Weapon_Impacts/Systems/Concrete/Concrete_Impact_Omni_01.Concrete_Impact_Omni_01")
        (Rendering|Decal|SpawnDecalatLocation "/Game/content/材质/弹孔贴花/弹孔贴花.弹孔贴花" "10.000000,10.000000,10.000000" (.Location (Collision|BreakHitResult _output_get)) (Math|Conversions|RotationFromXVector (.Normal (Collision|BreakHitResult _output_get))) 1e+01 :!label _label))
      (:SurfaceType1
        (Variables|Default|Set击中特效 "/Game/Weapon_Impacts/Systems/Metal/Metal_Impact_Directional_01.Metal_Impact_Directional_01")
        (goto _label))
      (:SurfaceType2
        (Variables|Default|Set击中特效 "/Game/Weapon_Impacts/Systems/Concrete/Concrete_Impact_Directional_01.Concrete_Impact_Directional_01")
        (goto _label))
      (:SurfaceType3
        (Variables|Default|Set击中特效 "/Game/Weapon_Impacts/Systems/Grass/Grass_Impact_Directional_01.Grass_Impact_Directional_01"))
      (:SurfaceType4
        (Variables|Default|Set击中特效 "/Game/Weapon_Impacts/Systems/Water/Water_Impact_Directional_01.Water_Impact_Directional_01"))
      (:SurfaceType5
        (Variables|Default|Set击中特效 "/Game/Weapon_Impacts/Systems/Wood/Impact_Wood_Directional_01.Impact_Wood_Directional_01")
        (goto _label))
      (:SurfaceType6
        (Variables|Default|Set击中特效 "/Game/Weapon_Impacts/Systems/Blood/Blood_Impact_Directional_01.Blood_Impact_Directional_01"))
      (:SurfaceType7
        (Variables|Default|Set击中特效 "/Game/Weapon_Impacts/Systems/Dirt/Dirt_Impact_Directional_01.Dirt_Impact_Directional_01")))
    (Effects|SpawnEmitteratLocation (Variables|Default|Get击中特效) (.Location (Collision|BreakHitResult _output_get)) (Math|Conversions|RotationFromXVector (.Normal (Collision|BreakHitResult _output_get))) "0.800000,0.800000,0.800000")
    (Networking|SwitchHasAuthority
      (:Authority
        (Game|Damage|ApplyPointDamage (.HitActor (Collision|BreakHitResult (Variables|Default|Get命中结果))) (Variables|Default|Get子弹伤害) (Transformation|GetActorLocation _伤害来源) (Variables|Default|Get命中结果) 0 _伤害来源))
      (:Remote
        _))
    (Utilities|FlowControl|Delay 0.2)
    (Actor|DestroyActor)))

(fn ConstructionScript)