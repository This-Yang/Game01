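; BP_装备的武器 is the equipped-weapon Blueprint, handling fire animation and recoil.
; One event plays the weapon's fire animation once on a supplied skeletal mesh.
; The recoil event restarts a timeline whose curve scales upward pitch input on player 0's pawn, alongside random yaw input on each forward update.
; Vertical and horizontal recoil strengths come from the weapon data asset.
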(event Custom|播放武器开火动画
  (params (播放的骨骼 :type Skeletal%20Mesh%20Component%20Object%20Reference))
  (Components|Animation|PlayAnimation 播放的骨骼 (Variables|Default|Get武器开火动画) false))

(event Custom|后坐力
  (bind _returnvalue (Game|Player|GetPlayerPawn 0))
  (bind _武器数据资产 (Variables|Default|Get武器数据资产))
  (bind _水平后坐力 (Variables|/Game/content/数据资产/武器数据资产/WP_数据资产.WP_数据资产_C|Get水平后坐力 _武器数据资产))
  (bind (_direction _后坐力变化) (Timeline|时间轴 PlayFromStart)
    (:Update
      (switch Utilities|FlowControl|Switch|SwitchonETimelineDirection _direction
        (:Forward
          (Pawn|Input|AddControllerPitchInput _returnvalue (* (Math|Float|Lerp 0.0 (Variables|/Game/content/数据资产/武器数据资产/WP_数据资产.WP_数据资产_C|Get垂直后坐力 _武器数据资产) _后坐力变化) -1.0))
          (Pawn|Input|AddControllerYawInput _returnvalue (Math|Random|RandomFloatinRange (* -1.0 _水平后坐力) _水平后坐力)))))))

(fn ConstructionScript)