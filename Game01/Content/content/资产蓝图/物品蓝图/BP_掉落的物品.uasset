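; Dropped item actor that appears in the world as a physics-simulated static mesh, defined by an item data asset.
; The construction script takes the mesh from that data asset, and BeginPlay turns on physics simulation.
; Highlight events (高亮显示, 关闭高亮) set and clear an interaction overlay material on the mesh.
; The 获取数据资产 (get data asset) function returns without any value wired.
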(event EventBeginPlay
  (Physics|SetSimulatePhysics (Variables|Default|GetStaticMesh) true))

(event Event关闭高亮
  (Rendering|Material|SetOverlayMaterial (Variables|Default|GetStaticMesh) 0 :!class /Script/Engine.MeshComponent))

(event Event高亮显示
  (Rendering|Material|SetOverlayMaterial (Variables|Default|GetStaticMesh) "/Game/content/材质/M_交互材质.M_交互材质" :!class /Script/Engine.MeshComponent))

(fn ConstructionScript
  (Components|StaticMesh|SetStaticMesh (Variables|Default|GetStaticMesh) (Variables|/Game/content/数据资产/物品数据资产/Item_数据资产.Item_数据资产_C|Get静态网格体 (Variables|Default|Get物品数据资产))))

(fn 获取数据资产
  (return 0))