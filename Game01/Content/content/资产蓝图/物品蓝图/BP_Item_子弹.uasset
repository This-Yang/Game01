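; Bullet item Blueprint (子弹) that adds rifle reserve ammo to the player character.
; On BeginPlay it casts player 0 to 主角01, adds its owned quantity (拥有的数量) to 步枪备单 and calls 更新子弹面板 to refresh the ammo panel.
; The usability check (是否可使用) always returns false, so the ammo is granted when the actor begins play, independent of that check.
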(event EventBeginPlay
  (bind _as主角_01 (Utilities|Casting|CastTo主角01 (Game|GetPlayerCharacter 0)))
  (Variables|/Game/content/人物/主角/主角01.主角01_C|Set步枪备单 _as主角_01 (+ (Variables|/Game/content/人物/主角/主角01.主角01_C|Get步枪备单 _as主角_01) (Variables|Default|Get拥有的数量)))
  (Default|更新子弹面板 _as主角_01))

(fn ConstructionScript
  (|CallParentFunction))

(fn 是否可使用
  (params (使用目标 :type 主角01%20Object%20Reference))
  (return false))